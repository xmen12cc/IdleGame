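; MainPlayer is the player Blueprint for what appears to be an idle game prototype, whose UI is the WB_FirstIdleTest widget.
; BeginPlay simply creates that widget and adds it to the viewport; Tick is empty.
; Disconnected graphs hold an inactive save/load system for slot "save1", mapping the widget's SpacePeople and Wood to the save's Asteroids and SpaceGoat, including a delayed save and first-time save creation.
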(event `self.ReceiveBeginPlay`
  (`|ExecutionSequence`
    (:`then_0`
      (bind _returnvalue (`|CreateWidget` "/Game/Blueprints/WB_FirstIdleTest.WB_FirstIdleTest_C"))
      (`UserWidget.AddToViewport` _returnvalue 0))))

(event `self.ReceiveTick`
  (params (DeltaSeconds :type "Float (single-precision)")))

(fn `UserConstructionScript`)